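; BP_PowerHandlePickup is a power handle on a power box that the player collects by walking into its trigger.
; On overlap with BP_Basic_Player it destroys the switch and trigger, flags the player as holding the handle, and shows the handle in the player's UI.
; It also powers off the linked GiantFan, turns the box's indicator and light red, and plays fan shutdown and switch sounds.
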(event `self.Trigger.OnComponentBeginOverlap`
  (params (OverlappedComponent :type "PrimitiveComponent Object Reference") (OtherActor :type "Actor Object Reference") (OtherComp :type "PrimitiveComponent Object Reference") (OtherBodyIndex :type Integer) (bFromSweep :type Boolean) (SweepResult :type "HitResult Structure (by ref)"))
  (bind _giantfan (`self.GiantFan`))
  (bind _returnvalue_location (`KismetMathLibrary.BreakTransform` (`SceneComponent.K2_GetComponentToWorld` (`/Game/BluePrints/BP_GiantFan.DefaultSceneRoot` _giantfan))))
  (cast `/Game/BluePrints/BP_Basic_Player` OtherActor)
  (`ActorComponent.K2_DestroyComponent` (`self.PowerSwitch`))
  (`ActorComponent.K2_DestroyComponent` (`self.Trigger`))
  (`/Game/BluePrints/BP_GiantFan.PowerOff` _giantfan)
  (set `/Game/BluePrints/BP_Basic_Player.HasPowerSwitch` true (`self.Player`))
  (`PrimitiveComponent.SetMaterial` (`self.PowerBox`) 3 "/Game/Materials/M_RedLight.M_RedLight")
  (`LightComponent.SetLightColor` (`self.PointLight`) (make `LinearColor` 1.0) true)
  (`GameplayStatics.SpawnSoundAtLocation` "/Game/Audio/GiantFan/FanPowerOffCue.FanPowerOffCue" _returnvalue_location (struct) 1.5 1.0 0.0 "/Game/Audio/GiantFan/FanAT.FanAT" null)
  (`Widget.SetVisibility` (`/Game/BluePrints/BP_MyUI.PowerHandle` (`/Game/BluePrints/BP_Basic_Player.MyUI` (`self.Player`))) "Visible")
  (`GameplayStatics.SpawnSoundAtLocation` "/Game/Audio/PowerSwitchSound.PowerSwitchSound" (`SceneComponent.K2_GetComponentLocation` (`self.PowerBox`)) (struct) 0.15 1.2 0.3 null null))

(fn `UserConstructionScript`)