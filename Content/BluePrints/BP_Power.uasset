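; BP_Power is a power box that shuts off steam when a player carrying the power switch walks up to it.
; Overlapping the Trigger checks HasPowerSwitch on BP_Basic_Player, then reveals the switch mesh.
; After a short delay, a timeline lerps the handle's relative rotation to flip it.
; When the timeline finishes, it calls TurnedOff on Steam and swaps a power box material to red.
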(event `self.ReceiveBeginPlay`
  (set `self.RotStart` (struct))
  (set `self.RotEnd` (struct :`Roll` 100.0)))

(event `self.Trigger.OnComponentBeginOverlap`
  (params (OverlappedComponent :type "PrimitiveComponent Object Reference") (OtherActor :type "Actor Object Reference") (OtherComp :type "PrimitiveComponent Object Reference") (OtherBodyIndex :type Integer) (bFromSweep :type Boolean) (SweepResult :type "HitResult Structure (by ref)"))
  (bind _asbp_basic_player (cast `/Game/BluePrints/BP_Basic_Player` OtherActor))
  (if (`/Game/BluePrints/BP_Basic_Player.HasPowerSwitch` _asbp_basic_player)
    (`SceneComponent.SetVisibility` (`self.PowerSwitch`) true false)
    (`KismetSystemLibrary.Delay` 0.5)
    (bind (_direction _rotation) (`Timeline|PowerSwitch Rotation` :!via `PlayFromStart`)
      (:`Update`
        (`SceneComponent.K2_SetRelativeRotation` (`self.SwitchHandle`) (`KismetMathLibrary.RLerp` (`self.RotStart`) (`self.RotEnd`) _rotation) false false))
      (:`Finished`
        (`/Game/BluePrints/BP_SteamObstacle.TurnedOff` (`self.Steam`))
        (`PrimitiveComponent.SetMaterial` (`self.PowerBox`) 3 "/Game/Materials/M_MachineRed.M_MachineRed")))))

(fn `UserConstructionScript`)