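; BP_Smasher is a crusher hazard that endlessly slams down and rises back up, flattening players caught beneath it.
; Two timelines lerp the mesh's relative Z from a start height captured in the construction script, triggering each other after short pauses.
; Box overlaps during descent squash a BP_Basic_Player's Cylinder, call the respawn dispatcher, then restore its transform after a delay.
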(event `SmasherDown`
  (bind _sm_smasher (`self.SM_Smasher`))
  (bind _smasherstart (`self.SmasherStart`))
  (bind _returnvalue (`SceneComponent.GetRelativeTransform` _sm_smasher))
  ;[1 1 1] Smasher Down
  (set `self.GoingDown?` true)
  (bind (_direction _newtrack_0) (`Timeline|ComingDown` :!via `PlayFromStart`)
    (:`Update`
      (`SceneComponent.K2_SetRelativeLocation` _sm_smasher (`KismetMathLibrary.MakeVector` (.x (.location _returnvalue)) (.y (.location _returnvalue)) (`KismetMathLibrary.Lerp` _smasherstart (- _smasherstart 44.0) _newtrack_0)) false false))
    (:`Finished`
      (set `self.GoingDown?` false)
      (`KismetSystemLibrary.Delay` 2.0)
      (`self.SmasherUp`))))

(event `self.ReceiveBeginPlay`
  ;[1 1 1] Begin the Smashing
  (`self.SmasherDown`))

(event `self.Box.OnComponentBeginOverlap`
  (params (OverlappedComponent :type "PrimitiveComponent Object Reference") (OtherActor :type "Actor Object Reference") (OtherComp :type "PrimitiveComponent Object Reference") (OtherBodyIndex :type Integer) (bFromSweep :type Boolean) (SweepResult :type "HitResult Structure (by ref)"))
  (if (`self.GoingDown?`)
    (bind _asbp_basic_player (cast `/Game/BluePrints/BP_Basic_Player` OtherActor))
    (`SceneComponent.K2_SetRelativeTransform` (`/Game/BluePrints/BP_Basic_Player.Cylinder` _asbp_basic_player) (`KismetMathLibrary.MakeTransform` (0.0 0.0 -80.0) (struct) (1.5 1.5 0.1)) false false)
    (`self.RespawnDispatcher`)
    (`KismetSystemLibrary.Delay` 3.0)
    (`SceneComponent.K2_SetRelativeTransform` (`/Game/BluePrints/BP_Basic_Player.Cylinder` _asbp_basic_player) (`KismetMathLibrary.MakeTransform` (0.0 0.0 0.0) (struct) (0.75 0.75 1.75)) false false)))

(event `SmasherUp`
  (bind _sm_smasher (`self.SM_Smasher`))
  (bind _smasherstart (`self.SmasherStart`))
  (bind _returnvalue (`SceneComponent.GetRelativeTransform` _sm_smasher))
  ;[1 1 1] Smasher Up
  (bind (_direction _newtrack_0) (`Timeline|GoingUp` :!via `PlayFromStart`)
    (:`Update`
      (`SceneComponent.K2_SetRelativeLocation` _sm_smasher (`KismetMathLibrary.MakeVector` (.x (.location _returnvalue)) (.y (.location _returnvalue)) (`KismetMathLibrary.Lerp` (- _smasherstart 44.0) _smasherstart _newtrack_0)) false false))
    (:`Finished`
      (`KismetSystemLibrary.Delay` 2.0)
      (`self.SmasherDown`))))

(fn `UserConstructionScript`
  (set `self.SmasherStart` (.z (.location (`SceneComponent.GetRelativeTransform` (`self.SM_Smasher`))))))