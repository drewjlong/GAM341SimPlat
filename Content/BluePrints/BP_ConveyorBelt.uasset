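; BP_ConveyorBelt is a conveyor belt that carries the player along while they overlap its Box trigger.
; Box overlap events filter for BP_Basic_Player, store it as the actor to move and toggle a touching flag.
; While the flag is set, Tick offsets that player along the Arrow component's forward vector at Speed, scaled by delta time and without sweeping for collision.
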(event `self.ReceiveTick`
  (params (DeltaSeconds :type "Float (single-precision)"))
  (if (`self.PlayerTouching`)
    (`self.K2_AddActorWorldOffset` (`self.ActorToMove`) (* (* (`SceneComponent.GetForwardVector` (`self.Arrow`)) (`self.Speed`)) DeltaSeconds) false false)))

(event `self.Box.OnComponentBeginOverlap`
  (params (OverlappedComponent :type "PrimitiveComponent Object Reference") (OtherActor :type "Actor Object Reference") (OtherComp :type "PrimitiveComponent Object Reference") (OtherBodyIndex :type Integer) (bFromSweep :type Boolean) (SweepResult :type "HitResult Structure (by ref)"))
  (bind _asbp_basic_player (cast `/Game/BluePrints/BP_Basic_Player` OtherActor))
  (set `self.ActorToMove` _asbp_basic_player)
  (set `self.PlayerTouching` true))

(event `self.Box.OnComponentEndOverlap`
  (params (OverlappedComponent :type "PrimitiveComponent Object Reference") (OtherActor :type "Actor Object Reference") (OtherComp :type "PrimitiveComponent Object Reference") (OtherBodyIndex :type Integer))
  (cast `/Game/BluePrints/BP_Basic_Player` OtherActor)
  (set `self.PlayerTouching` false))

(fn `UserConstructionScript`)