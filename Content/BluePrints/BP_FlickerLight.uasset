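; BP_FlickerLight is a light actor that flickers its PointLight at irregular intervals during play.
; From BeginPlay, an endless loop sets the light to a random intensity, waits, turns it off, and waits again.
; Min and max float variables bound both the random intensity and the random delay used for each on and off phase.
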(event `self.ReceiveBeginPlay`
  (`LightComponent.SetIntensity` (`self.PointLight`) (`KismetMathLibrary.RandomFloatInRange` (`self.MinFloatIntensity`) (`self.MaxFloatIntensity`)) :!label _label)
  (`KismetSystemLibrary.Delay` (`KismetMathLibrary.RandomFloatInRange` (`self.MinFloatDelay`) (`self.MaxFloatDelay`)))
  (`LightComponent.SetIntensity` (`self.PointLight`) 0.0)
  (`KismetSystemLibrary.Delay` (`KismetMathLibrary.RandomFloatInRange` (`self.MinFloatDelay`) (`self.MaxFloatDelay`)))
  (goto _label))

(fn `UserConstructionScript`)