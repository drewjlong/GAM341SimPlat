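; BP_SteamObstacle is a steam hazard that reacts to the player until it is turned off.
; It starts active, and while active an overlap with a BP_Basic_Player fires its Steam event dispatcher, leaving the response to bound listeners.
; The TurnedOff event clears the active flag, hides the particle effect and disables the box collision, with no path to switch it back on.
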(event `TurnedOff`
  (`KismetSystemLibrary.PrintString` "TurnedOff")
  (set `self.SteamOn` false)
  (`SceneComponent.SetVisibility` (`self.PS_FireNoSmoke`) false false)
  (`PrimitiveComponent.SetCollisionEnabled` (`self.Box`) "NoCollision"))

(event `self.ReceiveBeginPlay`
  (set `self.SteamOn` true))

(event `self.ReceiveActorBeginOverlap`
  (params (OtherActor :type "Actor Object Reference"))
  (if (`self.SteamOn`)
    (cast `/Game/BluePrints/BP_Basic_Player` OtherActor)
    (`self.SteamDispatcher`)))

(fn `UserConstructionScript`)